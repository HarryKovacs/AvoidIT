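; TriggerboxNote is a trigger actor that briefly shows a NoteReminder widget the first time something overlaps its Box.
; Begin overlap creates the widget and adds it to the viewport, then sets a PlayedOnce flag and prints a debug string.
; A one-second Delay removes the widget; end overlap feeds the same Delay when the widget reference is valid.
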(event `self.Box.OnComponentBeginOverlap`
  (params (OverlappedComponent :type "PrimitiveComponent Object Reference") (OtherActor :type "Actor Object Reference") (OtherComp :type "PrimitiveComponent Object Reference") (OtherBodyIndex :type Integer) (bFromSweep :type Boolean) (SweepResult :type "HitResult Structure (by ref)"))
  (if (not (`self.PlayedOnce`))
    (bind _returnvalue (`|CreateWidget` "/Game/Widgets/NoteReminder.NoteReminder_C"))
    (bind _output_get (set `self.NoteReminerRef` _returnvalue))
    (`UserWidget.AddToViewport` _output_get 0)
    (`|ExecutionSequence`
      (:`then_0`
        (`KismetSystemLibrary.Delay` 1.0 :!label _label)
        (`Widget.RemoveFromParent` (`self.NoteReminerRef`)))
      (:`then_1`
        (set `self.PlayedOnce` true)
        (`KismetSystemLibrary.PrintString` "sa")))))

(event `self.Box.OnComponentEndOverlap`
  (params (OverlappedComponent :type "PrimitiveComponent Object Reference") (OtherActor :type "Actor Object Reference") (OtherComp :type "PrimitiveComponent Object Reference") (OtherBodyIndex :type Integer))
  (if (`KismetSystemLibrary.IsValid` (`self.NoteReminerRef`))
    (goto _label)))

(fn `UserConstructionScript`)