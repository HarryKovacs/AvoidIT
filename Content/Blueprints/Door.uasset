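; Door actor that a first-person player opens and closes with the Interact input.
; An InteractBox overlap with BP_FirstPersonCharacter enables or disables input; both begin and end overlap set PlayerInRange true.
; Interact plays or reverses the OpenDoorTime timeline based on DoorOpen.
; Each timeline update toggles DoorOpen and lerps yaw through a half turn on a SceneCaptureComponent2D, rather than a door mesh.
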(event `InputAction|Interact`
  (params (Key :type "Key Structure"))
  (:`Pressed`
    (if (`self.bPlayerInRange`)
      (`self.Open Door`))))

(event `Open Door`
  ; Door Open/Close
  (if (`self.DoorOpen`)
    (bind (_direction _door) (`Timeline|OpenDoorTime` :!via `Reverse` :!label _label)
      (:`Update`
        (`SceneComponent.K2_SetRelativeRotation` (`self.SceneCaptureComponent2D`) (`KismetMathLibrary.MakeRotator` 0.0 0.0 (`KismetMathLibrary.Lerp` 0.0 -180.0 _door)) false false)
        (bind _output_get (set `self.DoorOpen` (not (stale _output_get))))))
    (else
      (goto _label))))

(event `self.InteractBox.OnComponentBeginOverlap`
  (params (OverlappedComponent :type "PrimitiveComponent Object Reference") (OtherActor :type "Actor Object Reference") (OtherComp :type "PrimitiveComponent Object Reference") (OtherBodyIndex :type Integer) (bFromSweep :type Boolean) (SweepResult :type "HitResult Structure (by ref)"))
  ; Enable Input
  (cast `/Game/FirstPerson/Blueprints/BP_FirstPersonCharacter` OtherActor)
  (set `self.bPlayerInRange` true)
  (`self.EnableInput` (`GameplayStatics.GetPlayerController` 0)))

(event `self.InteractBox.OnComponentEndOverlap`
  (params (OverlappedComponent :type "PrimitiveComponent Object Reference") (OtherActor :type "Actor Object Reference") (OtherComp :type "PrimitiveComponent Object Reference") (OtherBodyIndex :type Integer))
  ; Enable Input
  (cast `/Game/FirstPerson/Blueprints/BP_FirstPersonCharacter` OtherActor)
  (set `self.bPlayerInRange` true)
  (`self.DisableInput` (`GameplayStatics.GetPlayerController` 0)))

(fn `UserConstructionScript`)