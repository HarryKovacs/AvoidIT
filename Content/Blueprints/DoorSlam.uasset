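; DoorSlam is a one-shot trigger actor that throws two boxes and plays a door slam when its collision box is overlapped.
; The first overlap, if by the player, launches both boxes with physics force, then destroys them shortly afterwards.
; After a short delay, any overlap plays the sound at a hardcoded location and a timeline rolls SceneCaptureComponent2D, guarded by a DoOnce boolean.
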(event `self.Collisionbox.OnComponentBeginOverlap`
  (params (OverlappedComponent :type "PrimitiveComponent Object Reference") (OtherActor :type "Actor Object Reference") (OtherComp :type "PrimitiveComponent Object Reference") (OtherBodyIndex :type Integer) (bFromSweep :type Boolean) (SweepResult :type "HitResult Structure (by ref)"))
  (bind _box2 (`self.box2`))
  ; DoorSlam
  (`|ExecutionSequence`
    (:`then_0`
      ; BoxThrown
      (`/Engine/EditorBlueprintResources/StandardMacros.DoOnce` false
        (:`Completed`
          (if (== OtherActor (`GameplayStatics.GetPlayerCharacter` 0))
            (`PrimitiveComponent.SetSimulatePhysics` _box2 true)
            (`PrimitiveComponent.SetSimulatePhysics` (`self.box`) true)
            (`PrimitiveComponent.AddForce` _box2 (-850000.0 0.0 0.0) "None" false)
            (`PrimitiveComponent.AddForce` (`self.box`) (-850000.0 0.0 0.0) "None" false)
            (`KismetSystemLibrary.Delay` 1.6)
            (`ActorComponent.K2_DestroyComponent` _box2)
            (`ActorComponent.K2_DestroyComponent` (`self.box`))))))
    (:`then_1`
      (`KismetSystemLibrary.Delay` 1.0)
      (if (not (`self.DoOnce`))
        (`GameplayStatics.PlaySoundAtLocation` "/Game/Audio/DoorSlam.DoorSlam" (-1317.0 -425.0 1010.0) (struct) 1.0 1.0 0.0 null null null null)
        (bind (_direction _door) (`Timeline|Timeline_0`)
          (:`Update`
            (`SceneComponent.K2_SetRelativeRotation` (`self.SceneCaptureComponent2D`) (`KismetMathLibrary.MakeRotator` _door 0.0 20.0) false false)
            (set `self.DoOnce` true)))))))

(fn `UserConstructionScript`)