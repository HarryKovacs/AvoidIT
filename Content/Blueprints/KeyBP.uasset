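; Key pickup actor that the first-person character collects with the Interact input while nearby.
; A box trigger enables the actor's input and shows a Pickup prompt widget on entry, then reverses both on exit.
; Interacting plays a key sound and briefly shows a Key widget, then hides the key, removes the prompt and sets KeyCollected to block repeat pickups.
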(event `InputAction|Interact`
  (params (Key :type "Key Structure"))
  ; Pickup Interact
  (:`Pressed`
    (if (not (`self.KeyCollected`))
      (bind _returnvalue (`|CreateWidget` "/Game/Widgets/Key.Key_C"))
      (bind _output_get (set `self.KeyRef` _returnvalue))
      (`UserWidget.AddToViewport` _output_get 0)
      (`GameplayStatics.PlaySound2D` "/Game/Audio/llaves_5keys-5-338162.llaves_5keys-5-338162" 1.0 1.0 0.0 null null)
      (`KismetSystemLibrary.Delay` 0.5)
      ; Pickup
      (`Widget.RemoveFromParent` (`self.KeyRef`))
      (`self.SetActorHiddenInGame` (`self.Key`) true)
      (`Widget.RemoveFromParent` (`self.PickupRef`))
      (set `self.KeyCollected` true))))

(event `self.Box.OnComponentBeginOverlap`
  (params (OverlappedComponent :type "PrimitiveComponent Object Reference") (OtherActor :type "Actor Object Reference") (OtherComp :type "PrimitiveComponent Object Reference") (OtherBodyIndex :type Integer) (bFromSweep :type Boolean) (SweepResult :type "HitResult Structure (by ref)"))
  ; Enable Input
  (cast `/Game/FirstPerson/Blueprints/BP_FirstPersonCharacter` OtherActor)
  (set `self.PlayerInRange` true)
  (`self.EnableInput` (`GameplayStatics.GetPlayerController` 0))
  (if (not (`self.KeyCollected`))
    (bind _returnvalue (`|CreateWidget` "/Game/Widgets/Pickup.Pickup_C"))
    (bind _output_get (set `self.PickupRef` _returnvalue))
    (`UserWidget.AddToViewport` _output_get 0)))

(event `self.Box.OnComponentEndOverlap`
  (params (OverlappedComponent :type "PrimitiveComponent Object Reference") (OtherActor :type "Actor Object Reference") (OtherComp :type "PrimitiveComponent Object Reference") (OtherBodyIndex :type Integer))
  ; Enable Input
  (cast `/Game/FirstPerson/Blueprints/BP_FirstPersonCharacter` OtherActor)
  (set `self.PlayerInRange` false)
  (`self.DisableInput` (`GameplayStatics.GetPlayerController` 0))
  (`Widget.RemoveFromParent` (`self.PickupRef`)))

(fn `UserConstructionScript`)