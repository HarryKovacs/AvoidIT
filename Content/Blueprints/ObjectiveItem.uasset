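; ObjectiveItem is a collectible orb that the player picks up by overlap, with the last one opening the exit doors.
; Each pickup decrements TotalOrbs in BP_FirstPersonGameMode and shows the remaining count in a temporary WBP_RemainingCount widget.
; The orb hides immediately, then removes the widget and destroys itself after a short delay.
; The exit check counts live ObjectiveItem actors rather than TotalOrbs, then calls the left and right doors.
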(event `self.Sphere.OnComponentBeginOverlap`
  (params (OverlappedComponent :type "PrimitiveComponent Object Reference") (OtherActor :type "Actor Object Reference") (OtherComp :type "PrimitiveComponent Object Reference") (OtherBodyIndex :type Integer) (bFromSweep :type Boolean) (SweepResult :type "HitResult Structure (by ref)"))
  (bind _obj (`self.Obj`))
  (if (`self.ActorHasTag` OtherActor "Player")
    (bind _asbp_first_person_game_mode (cast `/Game/FirstPerson/Blueprints/BP_FirstPersonGameMode` (`GameplayStatics.GetGameMode`)))
    (bind _output_get (set `/Game/FirstPerson/Blueprints/BP_FirstPersonGameMode.TotalOrbs` (- (`/Game/FirstPerson/Blueprints/BP_FirstPersonGameMode.TotalOrbs` _asbp_first_person_game_mode) 1) _asbp_first_person_game_mode))
    (bind _returnvalue (`|CreateWidget` "/Game/Widgets/WBP_RemainingCount.WBP_RemainingCount_C" (`GameplayStatics.GetPlayerController` 0)))
    (bind _output_get_2 (set `self.RemainingCountWidgetRef` _returnvalue))
    (`UserWidget.AddToViewport` _output_get_2 0)
    (`/Game/Widgets/WBP_RemainingCount.UpdateCount` (`self.RemainingCountWidgetRef`) _output_get)
    (`|ExecutionSequence`
      (:`then_0`
        (`KismetSystemLibrary.PrintString` "orb collected")
        (`self.SetActorHiddenInGame` _obj true :!label _label)
        (`self.SetActorEnableCollision` _obj false)
        (`KismetSystemLibrary.Delay` 1.05)
        (`Widget.RemoveFromParent` (`self.RemainingCountWidgetRef`))
        (`self.K2_DestroyActor` (`self.Obj`)))
      (:`then_1`
        (bind _outactors (`GameplayStatics.GetAllActorsOfClass` "ObjectiveItem_C"))
        (if (== 1 (`KismetArrayLibrary.Array_Length` _outactors))
          (`KismetSystemLibrary.PrintString` "exit available")
          (`|ExecutionSequence`
            (:`then_0`
              (goto _label))
            (:`then_1`
              ; Exit Sequence
              (`|ExecutionSequence`
                (:`then_0`
                  (`/Game/Doors/RightDoor_BP.OpenRightDoor` (`self.RightDoor`)))
                (:`then_1`
                  (`/Game/Doors/LeftDoor_BP.OpenLeftDoor` (`self.LeftDoor`))))
              (`KismetSystemLibrary.PrintString` "doors open"))))))))

(fn `UserConstructionScript`)