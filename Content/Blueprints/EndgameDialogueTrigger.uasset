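; Trigger volume that shows the endgame widget once, on the first overlap of its box by any actor.
; If that first overlapping actor is a MonsterAI, it destroys the monster and opens the main menu level after 20 seconds.
; When an overlap ends while the stored widget is valid, it removes the widget from the viewport after a one-second delay.
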(event `self.Box.OnComponentBeginOverlap`
  (params (OverlappedComponent :type "PrimitiveComponent Object Reference") (OtherActor :type "Actor Object Reference") (OtherComp :type "PrimitiveComponent Object Reference") (OtherBodyIndex :type Integer) (bFromSweep :type Boolean) (SweepResult :type "HitResult Structure (by ref)"))
  (if (not (`self.PlayedOnce`))
    (bind _returnvalue (`|CreateWidget` "/Game/Widgets/EndgameWBP.EndgameWBP_C"))
    (bind _output_get (set `self.EndgameRef` _returnvalue))
    (`UserWidget.AddToViewport` _output_get 0)
    (set `self.PlayedOnce` true)
    (bind _asmonster_ai (cast `/Game/EnemyAI/MonsterAI` OtherActor))
    (`self.K2_DestroyActor` _asmonster_ai)
    (`KismetSystemLibrary.Delay` 20.0)
    (`GameplayStatics.OpenLevelBySoftObjectPtr` "/Game/Levels/MainMenu.MainMenu")))

(event `self.Box.OnComponentEndOverlap`
  (params (OverlappedComponent :type "PrimitiveComponent Object Reference") (OtherActor :type "Actor Object Reference") (OtherComp :type "PrimitiveComponent Object Reference") (OtherBodyIndex :type Integer))
  (if (`KismetSystemLibrary.IsValid` (`self.EndgameRef`))
    (`KismetSystemLibrary.Delay` 1.0)
    (`Widget.RemoveFromParent` (stale `self.Box.OnComponentBeginOverlap` _returnvalue))))

(fn `UserConstructionScript`)