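; BedNewLevel_BP is an interactable bed that sends the player to the Lvl_AvoidIT_Maze level.
; A Box overlap with BP_FirstPersonCharacter enables input on the bed and shows the BedInteract prompt widget; leaving reverses both.
; Pressing Interact starts a held camera fade, removes the prompt, calls DisableInput on the camera manager, then opens the maze after a fixed delay.
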(event `InputAction|Interact`
  (params (Key :type "Key Structure"))
  (bind _returnvalue (`GameplayStatics.GetPlayerController` 0))
  (bind _playercameramanager (`PlayerController.PlayerCameraManager` _returnvalue))
  ; Interaction
  (:`Pressed`
    (`PlayerCameraManager.StartCameraFade` :`self` _playercameramanager :`ToAlpha` 1.0 :`Duration` 1.4 :`bHoldWhenFinished` true)
    (`Widget.RemoveFromParent` (stale `self.Box.OnComponentBeginOverlap` _output_get))
    (`self.DisableInput` _playercameramanager _returnvalue)
    (`KismetSystemLibrary.Delay` 5.0)
    (`GameplayStatics.OpenLevelBySoftObjectPtr` "/Game/Levels/Lvl_AvoidIT_Maze.Lvl_AvoidIT_Maze")))

(event `self.Box.OnComponentBeginOverlap`
  (params (OverlappedComponent :type "PrimitiveComponent Object Reference") (OtherActor :type "Actor Object Reference") (OtherComp :type "PrimitiveComponent Object Reference") (OtherBodyIndex :type Integer) (bFromSweep :type Boolean) (SweepResult :type "HitResult Structure (by ref)"))
  ; Enable Input
  (cast `/Game/FirstPerson/Blueprints/BP_FirstPersonCharacter` OtherActor)
  (set `self.Player In Range` true)
  (`self.EnableInput` (`GameplayStatics.GetPlayerController` 0))
  (bind _returnvalue (`|CreateWidget` "/Game/Widgets/BedInteract.BedInteract_C"))
  (bind _output_get (set `self.BedInteractRef` _returnvalue))
  (`UserWidget.AddToViewport` _output_get 0))

(event `self.Box.OnComponentEndOverlap`
  (params (OverlappedComponent :type "PrimitiveComponent Object Reference") (OtherActor :type "Actor Object Reference") (OtherComp :type "PrimitiveComponent Object Reference") (OtherBodyIndex :type Integer))
  ; Enable Input
  (cast `/Game/FirstPerson/Blueprints/BP_FirstPersonCharacter` OtherActor)
  (set `self.Player In Range` false)
  (`self.DisableInput` (`GameplayStatics.GetPlayerController` 0))
  (`Widget.RemoveFromParent` (`self.BedInteractRef`)))

(fn `UserConstructionScript`)