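; Interactable notepad that the first-person player can read by holding Interact nearby.
; A box overlap enables the actor's own input and shows a ReadNote prompt, both cleared on exit.
; Pressing Interact disables character input and opens the Notepad widget, while releasing closes it, restores control and marks the note read.
; Leaving the box after reading briefly shows a NoteRead widget, guarded to play once.
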(event `InputAction|Interact`
  (params (Key :type "Key Structure"))
  (bind _returnvalue (`GameplayStatics.GetPlayerController` 0))
  ; Interact
  (:`Pressed`
    (set `self.InteractPressed` true)
    (bind _asbp_first_person_character (cast `/Game/FirstPerson/Blueprints/BP_FirstPersonCharacter` (`GameplayStatics.GetPlayerCharacter` 0)))
    (`self.DisableInput` _asbp_first_person_character _returnvalue)
    (if (`self.PlayerInRange`)
      (bind _returnvalue_2 (`|CreateWidget` "/Game/Widgets/Notepad.Notepad_C"))
      (bind _output_get (set `self.NoteRef` _returnvalue_2))
      (`UserWidget.AddToViewport` _output_get 0)))
  (:`Released`
    (`Widget.RemoveFromParent` (`self.NoteRef`))
    (`self.EnableInput` _asbp_first_person_character _returnvalue)
    (set `self.NoteRead` true)))

(event `self.Box.OnComponentBeginOverlap`
  (params (OverlappedComponent :type "PrimitiveComponent Object Reference") (OtherActor :type "Actor Object Reference") (OtherComp :type "PrimitiveComponent Object Reference") (OtherBodyIndex :type Integer) (bFromSweep :type Boolean) (SweepResult :type "HitResult Structure (by ref)"))
  ; Enable Input
  (cast `/Game/FirstPerson/Blueprints/BP_FirstPersonCharacter` OtherActor)
  (set `self.PlayerInRange` true)
  (`self.EnableInput` (`GameplayStatics.GetPlayerController` 0))
  ; Widget
  (bind _returnvalue (`|CreateWidget` "/Game/Widgets/ReadNote.ReadNote_C"))
  (bind _output_get (set `self.ReadNoteRef` _returnvalue))
  (`UserWidget.AddToViewport` _output_get 0)
  (if (`self.InteractPressed`)
    _))

(event `self.Box.OnComponentEndOverlap`
  (params (OverlappedComponent :type "PrimitiveComponent Object Reference") (OtherActor :type "Actor Object Reference") (OtherComp :type "PrimitiveComponent Object Reference") (OtherBodyIndex :type Integer))
  ; Enable Input
  (cast `/Game/FirstPerson/Blueprints/BP_FirstPersonCharacter` OtherActor)
  (set `self.PlayerInRange` false)
  (`self.DisableInput` (`GameplayStatics.GetPlayerController` 0))
  ; Remove Widget
  (`Widget.RemoveFromParent` (`self.ReadNoteRef`))
  (if (`self.NoteRead`)
    (if (not (`self.PlayedOnce`))
      (bind _returnvalue (`|CreateWidget` "/Game/Widgets/NoteRead.NoteRead_C"))
      (bind _output_get (set `self.NoteReadRef` _returnvalue))
      (`UserWidget.AddToViewport` _output_get 0)
      (`KismetSystemLibrary.Delay` 1.8)
      (`Widget.RemoveFromParent` _output_get)
      (set `self.PlayedOnce` true))))

(fn `UserConstructionScript`)