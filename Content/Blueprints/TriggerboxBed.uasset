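; Bed trigger volume that shows a BedReminder widget when its box is overlapped.
; The first begin overlap creates the widget and adds it to the viewport, and a PlayedOnce flag stops it from showing again.
; End overlap removes the stored widget if it is still valid.
; Neither event checks which actor overlaps the box.
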(event `self.Box.OnComponentBeginOverlap`
  (params (OverlappedComponent :type "PrimitiveComponent Object Reference") (OtherActor :type "Actor Object Reference") (OtherComp :type "PrimitiveComponent Object Reference") (OtherBodyIndex :type Integer) (bFromSweep :type Boolean) (SweepResult :type "HitResult Structure (by ref)"))
  (if (not (`self.PlayedOnce`))
    (bind _returnvalue (`|CreateWidget` "/Game/Widgets/BedReminder.BedReminder_C"))
    (bind _output_get (set `self.BedRef` _returnvalue))
    (`UserWidget.AddToViewport` _output_get 0)
    (set `self.PlayedOnce` true)))

(event `self.Box.OnComponentEndOverlap`
  (params (OverlappedComponent :type "PrimitiveComponent Object Reference") (OtherActor :type "Actor Object Reference") (OtherComp :type "PrimitiveComponent Object Reference") (OtherBodyIndex :type Integer))
  (if (`KismetSystemLibrary.IsValid` (`self.BedRef`))
    (`Widget.RemoveFromParent` (`self.BedRef`))))

(fn `UserConstructionScript`)