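; BP_Elevator is an elevator Blueprint that handles door toggling through its ToggleDoors_1 event.
; The event flips the DoorsAreClosed flag, and on opening plays the DoorLeft timeline to lerp the LeftDoor component's relative Y position outward while keeping its Z.
; The closing branch only sets the flag and ends in an empty Sequence, with no door movement or right-door logic wired.
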(event `ToggleDoors_1`
  (bind _leftdoor (`self.LeftDoor`))
  (bind (_relativelocation_x _relativelocation_y _relativelocation_z) (`KismetMathLibrary.BreakVector` (`SceneComponent.RelativeLocation` _leftdoor)))
  (if (`self.DoorsAreClosed?`)
    (set `self.DoorsAreClosed?` false)
    (`|ExecutionSequence`
      (:`then_0`
        (bind (_direction _doorfloat) (`Timeline|DoorLeft`)
          (:`Update`
            (`SceneComponent.K2_SetRelativeLocation` _leftdoor (`KismetMathLibrary.MakeVector` 0.0 (`KismetMathLibrary.Lerp` 0.0 -162.6 _doorfloat) _relativelocation_z) false false)))))
    (else
      (set `self.DoorsAreClosed?` true)
      (`|ExecutionSequence`))))

(fn `UserConstructionScript`)