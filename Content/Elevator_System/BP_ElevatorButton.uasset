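; Elevator call button that opens the elevator doors when the player presses Interact nearby, provided the key has been collected.
; A box overlap with the first-person character sets the range flag and toggles input on the button.
; With the key, it reveals a hidden actor, then uses timed delays to play a ding and open both doors with sound, guarded by HasSoundPlayed.
; Without the key, it briefly shows a KeyReminder widget.
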(event `InputAction|Interact`
  (params (Key :type "Key Structure"))
  (:`Pressed`
    (if (`self.bPlayerInRange`)
      (if (`self.HasSoundPlayed?`)
        _
        (elif (`/Game/Blueprints/KeyBP.KeyCollected` (`self.Keybp`))
          (`self.SetActorHiddenInGame` (`self.HiddenActor`) false)
          (`KismetSystemLibrary.Delay` 3.0)
          (`GameplayStatics.PlaySound2D` "/Game/Elevator_System/ElevatorDing.ElevatorDing" 1.0 1.0 0.0 null null)
          (set `self.HasSoundPlayed?` true)
          (`KismetSystemLibrary.Delay` 3.4)
          (`|ExecutionSequence`
            (:`then_0`
              (`/Game/Elevator_System/BP_LeftDoor.Open Left Door` (`self.LeftDoor`)))
            (:`then_1`
              (`/Game/Elevator_System/BP_RightDoor.Open Right Door` (`self.RightDoor`))))
          (if true
            (`GameplayStatics.PlaySound2D` "/Game/Elevator_System/ElevatorDoorOpening.ElevatorDoorOpening" 1.0 1.0 0.0 null null)
            (set `self.HasSoundPlayed?` true))
          (else
            (`KismetSystemLibrary.RetriggerableDelay` 0.4)
            (bind _returnvalue (`|CreateWidget` "/Game/Widgets/KeyReminder.KeyReminder_C"))
            (bind _output_get (set `self.KeyReminderREF` _returnvalue))
            (`UserWidget.AddToViewport` _output_get 0)
            (`KismetSystemLibrary.Delay` 0.3)
            (`Widget.RemoveFromParent` _output_get)))))))

(event `self.Box.OnComponentBeginOverlap`
  (params (OverlappedComponent :type "PrimitiveComponent Object Reference") (OtherActor :type "Actor Object Reference") (OtherComp :type "PrimitiveComponent Object Reference") (OtherBodyIndex :type Integer) (bFromSweep :type Boolean) (SweepResult :type "HitResult Structure (by ref)"))
  (cast `/Game/FirstPerson/Blueprints/BP_FirstPersonCharacter` OtherActor)
  (set `self.bPlayerInRange` true)
  (`self.EnableInput` (`GameplayStatics.GetPlayerController` 0)))

(event `self.Box.OnComponentEndOverlap`
  (params (OverlappedComponent :type "PrimitiveComponent Object Reference") (OtherActor :type "Actor Object Reference") (OtherComp :type "PrimitiveComponent Object Reference") (OtherBodyIndex :type Integer))
  (cast `/Game/FirstPerson/Blueprints/BP_FirstPersonCharacter` OtherActor)
  (set `self.bPlayerInRange` false)
  (`self.DisableInput` (`GameplayStatics.GetPlayerController` 0)))

(fn `UserConstructionScript`)