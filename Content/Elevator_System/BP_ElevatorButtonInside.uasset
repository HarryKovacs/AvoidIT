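; Elevator inside button that, on Interact, runs a scripted ride ending with the player teleported to a fixed new location.
; Box overlap toggles input for the button, though PlayerInRange is set true on both enter and exit.
; A delay-timed sequence closes both doors, fades the camera, teleports, then reopens the doors.
; It also plays a sound, reveals two hidden actors including a monster Easter egg, and sets HasSoundPlayed to block replays.
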(event `InputAction|Interact`
  (params (Key :type "Key Structure"))
  (bind _returnvalue (`GameplayStatics.GetPlayerCameraManager` 0))
  (bind _returnvalue_2 (`GameplayStatics.GetPlayerController` 0))
  (bind _playercameramanager (`PlayerController.PlayerCameraManager` _returnvalue_2))
  ; Elevator Button
  (:`Pressed`
    (if (`self.bPlayerInRange`)
      (if (not (`self.HasSoundPlayed`))
        (`self.SetActorHiddenInGame` (`self.HiddenActor`) false)
        (`KismetSystemLibrary.Delay` 1.0)
        (`|ExecutionSequence`
          (:`then_0`
            ; Elevator Doors Closing
            (`/Game/Elevator_System/BP_LeftDoor.Close Left Door` (`self.LeftDoor`))
            ; Camera Fade
            (`KismetSystemLibrary.Delay` 3.7 :!label _label)
            (`PlayerCameraManager.StartCameraFade` :`self` _playercameramanager :`ToAlpha` 1.0 :`Duration` 1.4 :`bHoldWhenFinished` true)
            (`self.DisableInput` _playercameramanager _returnvalue_2)
            (`KismetSystemLibrary.Delay` 5.0)
            ; New Elevator Spot
            (`self.K2_SetActorLocation` (`GameplayStatics.GetPlayerCharacter` 0) (910.0 -310.0 1010.0) false true)
            (`self.EnableInput` _returnvalue (`GameplayStatics.GetPlayerController` 0))
            (`PlayerCameraManager.StopCameraFade` _returnvalue)
            ; Elevator Doors Opening
            (`|ExecutionSequence`
              (:`then_0`
                (`/Game/Elevator_System/BP_LeftDoor.Open Left Door` (`self.LeftDoor`)))
              (:`then_1`
                (`/Game/Elevator_System/BP_RightDoor.Open Right Door` (`self.RightDoor`)))))
          (:`then_1`
            (`/Game/Elevator_System/BP_RightDoor.Close Right Door` (`self.RightDoor`))
            (goto _label))
          (:`then_2`
            ; Elevator Audio
            (`KismetSystemLibrary.Delay` 1.98)
            (`GameplayStatics.PlaySound2D` "/Game/Elevator_System/ElevatorDoorOpening.ElevatorDoorOpening" 1.0 1.0 0.0 null null)
            (set `self.HasSoundPlayed` true))
          (:`then_3`
            ; Monster Easter Egg
            (`KismetSystemLibrary.Delay` 1.97)
            (`self.SetActorHiddenInGame` (`self.AnotherHiddenActor`) false)))))))

(event `self.Box.OnComponentBeginOverlap`
  (params (OverlappedComponent :type "PrimitiveComponent Object Reference") (OtherActor :type "Actor Object Reference") (OtherComp :type "PrimitiveComponent Object Reference") (OtherBodyIndex :type Integer) (bFromSweep :type Boolean) (SweepResult :type "HitResult Structure (by ref)"))
  ; Enable Input
  (cast `/Game/FirstPerson/Blueprints/BP_FirstPersonCharacter` OtherActor)
  (set `self.bPlayerInRange` true)
  (`self.EnableInput` (`GameplayStatics.GetPlayerController` 0)))

(event `self.Box.OnComponentEndOverlap`
  (params (OverlappedComponent :type "PrimitiveComponent Object Reference") (OtherActor :type "Actor Object Reference") (OtherComp :type "PrimitiveComponent Object Reference") (OtherBodyIndex :type Integer))
  ; Enable Input
  (cast `/Game/FirstPerson/Blueprints/BP_FirstPersonCharacter` OtherActor)
  (set `self.bPlayerInRange` true)
  (`self.DisableInput` (`GameplayStatics.GetPlayerController` 0)))

(fn `UserConstructionScript`)