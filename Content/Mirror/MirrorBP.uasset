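; Interactable mirror that hands the player's view to a separate camera actor through a one-time fade.
; InteractBox overlap with the first-person character enables the mirror's input and shows an interact widget; leaving disables input and removes it.
; Pressing Interact removes the widget and, once only, fades the camera, disables pawn input, waits, then stops the fade and switches view target.
; Pawn input is not restored here.
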(event `InputAction|Interact`
  (params (Key :type "Key Structure"))
  (bind _returnvalue (`GameplayStatics.GetPlayerController` 0))
  (:`Pressed`
    (`|ExecutionSequence`
      (:`then_0`
        (if (`self.PlayerInRange`)
          (if (not (`self.DoOnce`))
            (`PlayerCameraManager.StartCameraFade` :`self` (`PlayerController.PlayerCameraManager` _returnvalue) :`ToAlpha` 1.0 :`Duration` 1.4 :`bHoldWhenFinished` true)
            (set `self.DoOnce` true)
            (`self.DisableInput` (`GameplayStatics.GetPlayerPawn` 0) _returnvalue)
            (`KismetSystemLibrary.Delay` 5.0)
            (`PlayerCameraManager.StopCameraFade` (`GameplayStatics.GetPlayerCameraManager` 0))
            (`PlayerController.SetViewTargetWithBlend` (`GameplayStatics.GetPlayerController` 0) (`self.CameraActor`) 0.0 "VTBlend_Linear" 0.0 true))))
      (:`then_1`
        (`Widget.RemoveFromParent` (`self.InteractRef`) :!label _label)))))

(event `self.InteractBox.OnComponentBeginOverlap`
  (params (OverlappedComponent :type "PrimitiveComponent Object Reference") (OtherActor :type "Actor Object Reference") (OtherComp :type "PrimitiveComponent Object Reference") (OtherBodyIndex :type Integer) (bFromSweep :type Boolean) (SweepResult :type "HitResult Structure (by ref)"))
  ; Enable Input
  (cast `/Game/FirstPerson/Blueprints/BP_FirstPersonCharacter` OtherActor)
  (set `self.PlayerInRange` true)
  (`self.EnableInput` (`GameplayStatics.GetPlayerController` 0))
  (bind _returnvalue (`|CreateWidget` "/Game/Widgets/Interact.Interact_C"))
  (bind _output_get (set `self.InteractRef` _returnvalue))
  (`UserWidget.AddToViewport` _output_get 0))

(event `self.InteractBox.OnComponentEndOverlap`
  (params (OverlappedComponent :type "PrimitiveComponent Object Reference") (OtherActor :type "Actor Object Reference") (OtherComp :type "PrimitiveComponent Object Reference") (OtherBodyIndex :type Integer))
  ; Enable Input
  (cast `/Game/FirstPerson/Blueprints/BP_FirstPersonCharacter` OtherActor)
  (set `self.PlayerInRange` true)
  (`self.DisableInput` (`GameplayStatics.GetPlayerController` 0))
  (goto _label))

(fn `UserConstructionScript`)